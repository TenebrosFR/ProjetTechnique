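; Build-mode component for the first-person character that previews and places the mesh selected in the inventory.
; While active, Tick traces from the camera to float the preview, rest it on hits, or attach it to an aimed MeshContainer, mirrored or offset by the aimed side.
; A bounds sphere overlap tints the preview red or green.
; Inputs toggle the mode, rotate yaw, and spawn a MeshContainer at the preview, regardless of overlap.
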(event `self.ReceiveTick`
  (params (DeltaSeconds :type "Float (single-precision)"))
  (if (`self.IsBuildMode`)
    (`self.PreviewLoop`)))

(event `PreviewLoop`
  (bind (_returnvalue_location _returnvalue_rotation) (`KismetMathLibrary.BreakTransform` (`SceneComponent.K2_GetComponentToWorld` (`self.First Person Camera`))))
  (bind (_outhit _returnvalue) (`KismetSystemLibrary.LineTraceSingle` _returnvalue_location (+ _returnvalue_location (* (`KismetMathLibrary.GetForwardVector` _returnvalue_rotation) (`self.Build Range`))) "TraceTypeQuery3"))
  (`|ExecutionSequence`
    (:`then_0`
      (`self.IsDifferentSelectedMesh`
        (:`true`
          (`self.SetStaticMesh` (`/Game/Widget/Inventory.SelectedMesh` (`/Game/FirstPerson/Blueprints/BP_FirstPersonCharacter.Inventory` (`self.First Person Character`)))))))
    (:`then_1`
      (`self.UpdateMesh` _outhit _returnvalue))
    (:`then_2`
      (`self.CheckMeshBounds`))))

(event `EnhancedInput|/Game/FirstPerson/Input/Actions/IA_AcceptBuild`
  (params (ActionValue :type Boolean) (ElapsedSeconds :type "Float (double-precision)") (TriggeredSeconds :type "Float (double-precision)") (InputAction :type "InputAction Object Reference" :default "/Game/FirstPerson/Input/Actions/IA_AcceptBuild.IA_AcceptBuild"))
  (:`Triggered`
    (bind _returnvalue (`|SpawnActorFromClass` "/Game/Blueprint/MeshContainer.MeshContainer_C" (`SceneComponent.K2_GetComponentToWorld` (`self.PreviewMesh`)) "Undefined" "MultiplyWithRoot" null null))
    (`StaticMeshComponent.SetStaticMesh` (`/Game/Blueprint/MeshContainer.StaticMesh` _returnvalue) (`self.Selected Mesh`))))

(event `EnhancedInput|/Game/FirstPerson/Input/Actions/IA_BuildingRotation`
  (params (ActionValue :type Boolean) (ElapsedSeconds :type "Float (double-precision)") (TriggeredSeconds :type "Float (double-precision)") (InputAction :type "InputAction Object Reference" :default "/Game/FirstPerson/Input/Actions/IA_BuildingRotation.IA_BuildingRotation"))
  (:`Ongoing`
    (`self.AddRotation`)))

(event `EnhancedInput|/Game/FirstPerson/Input/Actions/IA_Build`
  (params (ActionValue :type Boolean) (ElapsedSeconds :type "Float (double-precision)") (TriggeredSeconds :type "Float (double-precision)") (InputAction :type "InputAction Object Reference" :default "/Game/FirstPerson/Input/Actions/IA_Build.IA_Build"))
  (:`Started`
    (`/Engine/EditorBlueprintResources/StandardMacros.FlipFlop`
      (:`A`
        (set `self.IsBuildMode` true))
      (:`B`
        (set `self.IsBuildMode` false)
        (`self.SetStaticMesh` null)))))

(event `self.ReceiveBeginPlay`
  (bind _asbp_first_person_character (cast `/Game/FirstPerson/Blueprints/BP_FirstPersonCharacter` (`self.GetOwner`)))
  (bind _output_get (set `self.First Person Character` _asbp_first_person_character))
  (set `self.First Person Camera` (`/Game/FirstPerson/Blueprints/BP_FirstPersonCharacter.FirstPersonCamera` _output_get))
  (bind _returnvalue (`|SpawnActorFromClass` "/Game/Blueprint/MeshContainer.MeshContainer_C" (`self.BuildPreviewTransform`) "Undefined" "MultiplyWithRoot" null null))
  (bind _output_get_2 (set `self.PreviewMeshContainer` _returnvalue))
  (set `self.PreviewMesh` (`/Game/Blueprint/MeshContainer.StaticMesh` _output_get_2)))

(fn `AddRotation`
  (locals (Rotation :type "Float (double-precision)"))
  (bind (_rotationadded_roll _rotationadded_pitch _rotationadded_yaw) (`KismetMathLibrary.BreakRotator` (`self.RotationAdded`)))
  (bind _output_get (set `local.Rotation` (+ _rotationadded_yaw 1.0)))
  (if (> _output_get 360.0)
    (set `local.Rotation` (- (`local.Rotation`) 360.0)))
  (set `self.RotationAdded` (`KismetMathLibrary.MakeRotator` _rotationadded_roll _rotationadded_pitch (`local.Rotation`))))

(fn `CheckMeshBounds`
  (bind _previewmesh (`self.PreviewMesh`))
  (bind _previewmesh_2 (`self.PreviewMesh`))
  (bind _previewmesh_3 (`self.PreviewMesh`))
  (bind _staticmesh (`StaticMeshComponent.StaticMesh` _previewmesh_3)
    (:`then`
      (bind (_returnvalue_origin _returnvalue_boxextent _returnvalue_sphereradius) (`KismetMathLibrary.BreakBoxSphereBounds` (`StaticMesh.GetBounds` _staticmesh)))
      (bind _outcomponents (`KismetSystemLibrary.SphereOverlapComponents` _returnvalue_origin _returnvalue_sphereradius (`|MakeArray` "ObjectTypeQuery1" :!type "EObjectTypeQuery Enum") "/Script/Engine.StaticMesh" (`|MakeArray` (`self.GetOwner` _previewmesh_3))))
      (if (> (`KismetArrayLibrary.Array_Length` _outcomponents) 0)
        (for (_ _array_index) (`MeshComponent.GetMaterials` _previewmesh)
          (`PrimitiveComponent.SetMaterial` _previewmesh _array_index "/Game/Material/M_TransparentRed.M_TransparentRed"))
        (else
          (for (_ _array_index_2) (`MeshComponent.GetMaterials` _previewmesh_2)
            (`PrimitiveComponent.SetMaterial` _previewmesh_2 _array_index_2 "/Game/Material/M_TransparentGreen.M_TransparentGreen")))))
    (:`else`)))

(fn `SetStaticMesh`
  (params (`Selected Mesh` :type "StaticMesh Object Reference"))
  (returns (`Static Mesh` :type "StaticMesh Object Reference"))
  (bind _previewmesh (`self.PreviewMesh`))
  (bind _output_get (set `self.Selected Mesh` `Selected Mesh`))
  (`StaticMeshComponent.SetStaticMesh` _previewmesh _output_get)
  (set `self.RotationAdded` (struct))
  (return (`StaticMeshComponent.StaticMesh` _previewmesh)))

(fn `UpdateMesh`
  (params (Hit :type "HitResult Structure (by ref)") (IsHit :type Boolean))
  (locals (IsBehindMesh :type Boolean) (Multiplier :type "Float (double-precision)") (PivotPosition :type "Float (double-precision)"))
  (bind (_bblockinghit _binitialoverlap _time _distance _location _impactpoint _normal _impactnormal _physmat _hitactor) (`GameplayStatics.BreakHitResult` Hit))
  (bind _previewmeshcontainer (`self.PreviewMeshContainer`))
  (bind _previewmesh (`self.PreviewMesh`))
  (bind _previewmeshcontainer_2 (`self.PreviewMeshContainer`))
  (bind _first_person_camera (`self.First Person Camera`))
  (bind (_returnvalue_x _returnvalue_y _returnvalue_z) (`KismetMathLibrary.BreakVector` (`SceneComponent.K2_GetComponentLocation` _first_person_camera)))
  (bind (_returnvalue_x_2 _returnvalue_y_2) (`KismetMathLibrary.BreakVector` (+ (* (`SceneComponent.GetForwardVector` _first_person_camera) (`self.Build Range`)) (`KismetMathLibrary.MakeVector` _returnvalue_x _returnvalue_y _returnvalue_z))))
  (if (== _hitactor _previewmeshcontainer_2)
    (`/Engine/EditorBlueprintResources/StandardMacros.IsValid` (`Actor.GetAttachParentActor` _previewmeshcontainer_2)
      (:`Is Valid`
        (`SceneComponent.K2_SetRelativeRotation` (`self.PreviewMesh`) (`self.RotationAdded`) false false))
      (:`Is Not Valid`
        (`Actor.K2_DetachFromActor` (`self.PreviewMeshContainer`) "KeepRelative" "KeepRelative" "KeepRelative" :!label _label)
        (`SceneComponent.K2_SetRelativeTransform` (`self.PreviewMesh`) (`KismetMathLibrary.MakeTransform` (`KismetMathLibrary.MakeVector` _returnvalue_x_2 _returnvalue_y_2) (`self.RotationAdded`)) false false)))
    (elif IsHit
      (`self.Selected Mesh`
        (:`then`
          (bind _asmesh_container (cast `/Game/Blueprint/MeshContainer` _hitactor)
            (:`then`
              (bind _staticmesh (`/Game/Blueprint/MeshContainer.StaticMesh` _asmesh_container))
              (if (not (== (`SceneComponent.GetAttachParent` (`Actor.RootComponent` _previewmeshcontainer)) _staticmesh))
                (`Actor.K2_AttachToComponent` _previewmeshcontainer _staticmesh "None" "KeepRelative" "KeepRelative" "KeepRelative" false)
                (set `self.RotationAdded` (struct)))
              (bind _returnvalue_x_3 (`KismetMathLibrary.BreakVector` (/ (`.BoxExtent` (`KismetSystemLibrary.GetComponentBounds` _staticmesh)) 2.0)))
              (bind _returnvalue (> _returnvalue_x_3 (.x (`KismetMathLibrary.InverseTransformLocation` (`SceneComponent.K2_GetComponentToWorld` _staticmesh) _location))))
              (if (!= (`self.IsAimingToLeftSide`) _returnvalue)
                (set `self.RotationAdded` (struct)))
              (set `self.IsAimingToLeftSide` _returnvalue)
              (if (`self.IsAimingToLeftSide`)
                (`SceneComponent.K2_SetRelativeTransform` _previewmesh (`KismetMathLibrary.MakeTransform` (0.0 0.0 0.0) (`self.RotationAdded`) (-1.0 1.0 1.0)) false false)
                (else
                  (bind (_relativelocation_x _relativelocation_y _relativelocation_z) (`KismetMathLibrary.BreakVector` (`SceneComponent.RelativeLocation` _staticmesh)))
                  (`SceneComponent.K2_SetRelativeTransform` _previewmesh (`KismetMathLibrary.MakeTransform` (`KismetMathLibrary.MakeVector` (+ _relativelocation_x (.x (`.Max` (`StaticMeshComponent.GetLocalBounds` (`self.PreviewMesh`))))) _relativelocation_y _relativelocation_z) (`self.RotationAdded`)) false false))))
            (:`CastFailed`
              (`SceneComponent.K2_SetRelativeTransform` (`self.PreviewMesh`) (`KismetMathLibrary.MakeTransform` (`KismetMathLibrary.MakeVector` (.x _location) (.y _location)) (`self.RotationAdded`)) false false))))
        (:`else`))
      (else
        (goto _label)))))